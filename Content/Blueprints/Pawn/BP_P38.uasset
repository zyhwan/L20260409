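; BP_P38 is a player-controlled P-38 aircraft pawn that flies forward constantly and fires rockets.
; Tick adds movement input along the actor's forward vector, so steering comes purely from changing orientation.
; Pitch and Roll axes apply local rotation scaled by RotationSpeed and frame delta time.
; The Fire action calls a Fire function that spawns BP_Rocket at the Arrow component's world transform.
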(event `self.ReceiveTick`
  (params (DeltaSeconds :type "Float (single-precision)"))
  (`self.AddMovementInput` (`self.GetActorForwardVector`)))

(event `InputAxis|Pitch`
  (params (AxisValue :type "Float (single-precision)"))
  (`self.K2_AddActorLocalRotation` (`KismetMathLibrary.MakeRotator` 0.0 (* AxisValue (`GameplayStatics.GetWorldDeltaSeconds`) (`self.RotationSpeed`)))))

(event `InputAction|Fire`
  (params (Key :type "Key Structure"))
  (:`Pressed`
    (`self.Fire`)))

(event `InputAxis|Roll`
  (params (AxisValue :type "Float (single-precision)"))
  (`self.K2_AddActorLocalRotation` (`KismetMathLibrary.MakeRotator` (* AxisValue (`GameplayStatics.GetWorldDeltaSeconds`) (`self.RotationSpeed`)))))

(fn `Fire`
  (`|SpawnActorFromClass` "/Game/Blueprints/Pawn/BP_Rocket.BP_Rocket_C" (`SceneComponent.K2_GetComponentToWorld` (`self.Arrow`)) "Undefined" "MultiplyWithRoot" null null))

(fn `UserConstructionScript`)