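; BP_Controller is a controller Blueprint holding unconnected logic for rotating player 0's pawn.
; Two event graph chains would add local roll and pitch rotation, scaled by frame delta time and RotationSpeed.
; Neither chain has a triggering event and both multiply by a literal zero, so they never run or produce rotation.
; The construction script is empty.
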(fn `UserConstructionScript`)